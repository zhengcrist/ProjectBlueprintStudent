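; Double door Blueprint whose two mesh leaves swing open and closed in mirrored yaw by RotationAngle.
; The OpenDoor event toggles IsClosed and plays or reverses a Timeline that drives both leaf rotations.
; The construction script poses the leaves and sets the Timeline position from IsClosed, so a door can start open or closed.
; Disconnected leftover nodes hold an older instant-snap toggle that never runs.
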(event Custom|OpenDoor
  (if (Variables|Default|GetIsClosed)
    (Variables|Default|SetIsClosed false)
    (bind _rotationvalue (Timeline|Timeline Play)
      (:Update
        (Transformation|SetRelativeRotation (Variables|Default|GetDoor_3_StaticMeshComponent0) (Math|Rotator|MakeRotator 0.0 0.0 (* _rotationvalue (Variables|Default|GetRotationAngle) -1.0)) false false)
        (Transformation|SetRelativeRotation (Variables|Default|GetDoor_3_StaticMeshComponent1) (Math|Rotator|MakeRotator 0.0 0.0 (Math|Float|Lerp 1.8e+02 (+ (Variables|Default|GetRotationAngle) 1.8e+02) _rotationvalue)) false false)))
    (else
      (Variables|Default|SetIsClosed true)
      (Timeline|Timeline Reverse))))

(event EventBeginPlay)

(event Collision|EventActorBeginOverlap
  (params (OtherActor :type Actor%20Object%20Reference)))

(event EventTick
  (params (DeltaSeconds :type Float%20%28single-precision%29)))

(fn ConstructionScript
  (Transformation|SetRelativeRotation (Variables|Default|GetDoor_3_StaticMeshComponent1) (Math|Rotator|MakeRotator 0.0 0.0 (select (Variables|Default|GetIsClosed) 1.8e+02 (+ (Variables|Default|GetRotationAngle) 1.8e+02))) false false)
  (Transformation|SetRelativeRotation (Variables|Default|GetDoor_3_StaticMeshComponent0) (Math|Rotator|MakeRotator 0.0 0.0 (select (Variables|Default|GetIsClosed) 0.0 (* (Variables|Default|GetRotationAngle) -1.0))) false false)
  (Components|Timeline|SetNewTime (Variables|Default|GetTimeline) (select (Variables|Default|GetIsClosed) 0.0 2.0)))